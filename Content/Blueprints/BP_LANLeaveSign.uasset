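; LAN leave sign actor that animates its static mesh vertically to the stored BeginLOC height.
; The Move timeline lerps from the mesh's current Z toward that height each update, leaving X and Y unchanged.
; BeginMove plays it on demand, and BeginPlay plays it automatically outside lobby levels when GI_InfoStorage reports HasSeenStart.
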(event EventBeginPlay
  (bind _staticmeshcomponent (Variables|Debug|GetStaticMeshComponent))
  (bind _returnvalue (Transformation|GetWorldLocation _staticmeshcomponent))
  (bind _returnvalue_2 (Game|GetCurrentLevelName true))
  (if (not (Utilities|String|Contains _returnvalue_2 "lobby"))
    (bind _asgi_info_storage (Utilities|Casting|CastToGI_InfoStorage (Game|GetGameInstance)))
    (if (Variables|/Game/Blueprints/GI_InfoStorage.GI_InfoStorage_C|GetHasSeenStart _asgi_info_storage)
      (bind _move (Timeline|Move Play)
        (:Update
          (Transformation|SetWorldLocation (Variables|Debug|GetStaticMeshComponent) (Math|Vector|Lerp(Vector) (Math|Vector|MakeVector (.x _returnvalue) (.y _returnvalue) (.z _returnvalue)) (Math|Vector|MakeVector (.x _returnvalue) (.y _returnvalue) (.z (Variables|Default|GetBeginLOC))) _move) false false))))))

(event EventBeginMove
  (bind _staticmeshcomponent (Variables|Debug|GetStaticMeshComponent))
  (bind _returnvalue (Transformation|GetWorldLocation _staticmeshcomponent))
  (bind _move (Timeline|Move Play)
    (:Update
      (Transformation|SetWorldLocation (Variables|Debug|GetStaticMeshComponent) (Math|Vector|Lerp(Vector) (Math|Vector|MakeVector (.x _returnvalue) (.y _returnvalue) (.z _returnvalue)) (Math|Vector|MakeVector (.x _returnvalue) (.y _returnvalue) (.z (Variables|Default|GetBeginLOC))) _move) false false))))

(fn ConstructionScript)