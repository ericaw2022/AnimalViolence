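; BP_SpikeRotator is a rotating hazard that damages actors hit by its two beams.
; Three self-restarting timelines lerp the relative rotation of the base mesh and both beam scene components from BeginPlay.
; On authority, Hit passes a one-second DoOnce gate, then sends TakeDamageMessage only for beam contacts, so other contacts also consume the cooldown.
; Every hit also prints a leftover "Hello" debug string.
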(event Custom|Event%20Rotate%20Base
  ;[0.15 0.15 0.15 0.5] Rots
  (bind _turn (Timeline|Rotate PlayFromStart)
    (:Update
      (Transformation|SetRelativeRotation (Variables|Debug|GetStaticMeshComponent) (Math|Rotator|Lerp(Rotator) (Variables|Default|GetIntROT) (Variables|Default|GetFinROT) _turn) false false))
    (:Finished
      (CallFunction|EventRotateBase))))

(event Custom|RotateBeam2
  ;[0.15 0.15 0.15 0.5] Rots
  (bind _spin (Timeline|Timeline PlayFromStart)
    (:Update
      (Transformation|SetRelativeRotation (Variables|Default|GetBeamScene2) (Math|Rotator|Lerp(Rotator) (Variables|Default|GetIntSpin_0) (Variables|Default|GetFinSpin_0) _spin) false false))
    (:Finished
      (CallFunction|RotateBeam2))))

(event Custom|RotateBeam1
  ;[0.15 0.15 0.15 0.5] Rots
  (bind _spin (Timeline|Spin PlayFromStart)
    (:Update
      (Transformation|SetRelativeRotation (Variables|Default|GetBeamScene) (Math|Rotator|Lerp(Rotator) (Variables|Default|GetIntSpin) (Variables|Default|GetFinSpin) _spin) false false))
    (:Finished
      (CallFunction|RotateBeam1))))

(event Custom|OpenGate
  ;[0.15 0.15 0.15 0.5] damage
  (Utilities|FlowControl|DoOnce false) ; enters at Reset
)

(event EventBeginPlay
  ;[0.15 0.15 0.15 0.5] begin play
  (CallFunction|EventRotateBase)
  (CallFunction|RotateBeam1)
  (CallFunction|RotateBeam2))

(event Collision|EventHit
  (params (MyComp :type Primitive%20Component%20Object%20Reference) (Other :type Actor%20Object%20Reference) (OtherComp :type Primitive%20Component%20Object%20Reference) (bSelfMoved :type Boolean) (HitLocation :type Vector :default "0, 0, 0") (HitNormal :type Vector :default "0, 0, 0") (NormalImpulse :type Vector :default "0, 0, 0") (Hit :type Hit%20Result%20Structure%20%28by%20ref%29))
  ;[0.15 0.15 0.15 0.5] damage
  (Development|PrintString "Hello")
  (Networking|SwitchHasAuthority
    (:Authority
      (Utilities|FlowControl|DoOnce false
        (:Completed
          (Utilities|Time|SetTimerbyEvent (delegate Custom|OpenGate) 1.0)
          (if (or (== MyComp (Variables|Default|GetBeam)) (== MyComp (Variables|Default|GetBeam2)))
            (Class|BPIDamagable|TakeDamage(Message) Other (Utilities|Struct|MakeS_DamageInfo 25.0 "NewEnumerator4" "NewEnumerator1" false false true true) HitNormal HitLocation)))))))

(fn ConstructionScript)