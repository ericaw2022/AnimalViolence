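; BP_Melee_Master is a melee weapon component, apparently the base for melee weapons, that sets up an optional weapon trail effect.
; On BeginPlay, if UsesTrail is set, it attaches an inactive Niagara system midway between its TrailBegin and TrailEnd sockets, oriented along the line between them.
; It stores the system and sets TrailWidth to the socket distance; activation is not handled in this graph.
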(event EventBeginPlay
  (bind _self self)
  (bind _returnvalue (Transformation|GetSocketLocation _self "TrailBegin"))
  (bind _returnvalue_2 (Transformation|GetSocketLocation _self "TrailEnd"))
  (bind _returnvalue_3 (- _returnvalue _returnvalue_2))
  (|CallParentFunction)
  (if (Variables|Default|GetUsesTrail?)
    (bind _returnvalue_4 (Niagara|SpawnSystemAttached (Variables|Default|GetWeaponTrail) self "None" (/ (+ _returnvalue _returnvalue_2) 2.0) (Math|Rotator|MakeRotfromZ _returnvalue_3) "KeepWorldPosition" false false))
    (bind _output_get (Variables|Default|SetWeaponTrailComp _returnvalue_4))
    (Effects|Components|ParticleSystem|SetFloatParameter _output_get "TrailWidth" (Math|Vector|VectorLength _returnvalue_3))))

(event EventTick
  (params (DeltaSeconds :type Float%20%28single-precision%29))
  (|CallParentFunction DeltaSeconds) ; This node is disabled and will not be called.\nDrag off pins to build functionality.
)