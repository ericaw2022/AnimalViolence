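; Base projectile firing component for weapons, providing the Shoot function that launches a projectile from the instigating player.
; Shoot spawns the configured ProjectileActor class at the location and rotation of a named socket on the Instigator's mesh.
; It passes itself as MyWeapon and the Instigator as InstigatingPlayer, then calls Shot on the spawned actor with the socket name.
; The event graph has no active logic.
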(event EventBeginPlay
  (|CallParentFunction) ; This node is disabled and will not be called.\nDrag off pins to build functionality.
)

(event EventTick
  (params (DeltaSeconds :type Float%20%28single-precision%29))
  (|CallParentFunction DeltaSeconds) ; This node is disabled and will not be called.\nDrag off pins to build functionality.
)

(fn Shoot
  (params (Instigator :type BP%20Combat%20Character%20Object%20Reference))
  (bind _projectilesocketname (Variables|Default|GetProjectileSocketName))
  (bind _mesh (Variables|/Script/Engine.Character|GetMesh Instigator))
  (bind _returnvalue (Game|SpawnActorfromClass (Variables|Default|GetProjectileActor) (Math|Transform|MakeTransform (Transformation|GetSocketLocation _mesh _projectilesocketname) (Transformation|GetSocketRotation _mesh _projectilesocketname) "1.000000,1.000000,1.000000") "Undefined" "MultiplyWithRoot" 0 self Instigator 0))
  (Default|Shot _returnvalue (Variables|Default|GetProjectileSocketName))
  (return))