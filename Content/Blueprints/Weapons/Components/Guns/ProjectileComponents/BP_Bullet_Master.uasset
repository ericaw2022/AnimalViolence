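; Master bullet projectile for guns that sticks to whatever it hits and deals the firing weapon's damage.
; The first hit attaches it to the struck component, at a spine socket for BP_CombatCharacter, and disables projectile collision.
; After DamageDelay it spawns an impact effect and sends a damage message built from MyWeapon's settings.
; It calls HitsUpdate on the instigating player if damage succeeds, then destroys itself shortly afterward.
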(event Custom|DestroyProjectile
  (Utilities|FlowControl|Delay 0.2)
  (Actor|DestroyActor))

(event Collision|EventHit
  (params (MyComp :type Primitive%20Component%20Object%20Reference) (Other :type Actor%20Object%20Reference) (OtherComp :type Primitive%20Component%20Object%20Reference) (bSelfMoved :type Boolean) (HitLocation :type Vector :default "0, 0, 0") (HitNormal :type Vector :default "0, 0, 0") (NormalImpulse :type Vector :default "0, 0, 0") (Hit :type Hit%20Result%20Structure%20%28by%20ref%29))
  (bind (_bblockinghit _binitialoverlap _time _distance _location _impactpoint _normal _impactnormal _physmat _hitactor) (Collision|BreakHitResult Hit))
  (bind _myweapon (Variables|Default|GetMyWeapon))
  (Utilities|FlowControl|DoOnce false
    (:Completed
      (if (== (Utilities|GetClass Other) "/Game/Variant_Combat/Blueprints/BP_CombatCharacter.BP_CombatCharacter_C")
        (Transformation|AttachComponentToComponent MyComp OtherComp "ORG-spine_003" "KeepWorld" "KeepWorld" "KeepWorld" true)
        (else
          (Transformation|AttachComponentToComponent MyComp OtherComp "None" "KeepWorld" "KeepWorld" "KeepWorld" true)))
      (Collision|SetCollisionEnabled (Variables|Default|GetProjectile) "NoCollision")
      (Utilities|FlowControl|Delay (Variables|Default|GetDamageDelay))
      (Niagara|SpawnSystematLocation (Variables|Default|GetParticle) (Transformation|GetActorLocation))
      (bind _wasdamaged_ (Class|BPIDamagable|TakeDamage(Message) _hitactor (Utilities|Struct|MakeS_DamageInfo (Variables|/Game/Blueprints/Weapons/Components/BP_Weapons_Master_Component.BP_Weapons_Master_Component_C|GetDamageAmount _myweapon) (Variables|/Game/Blueprints/Weapons/Components/BP_Weapons_Master_Component.BP_Weapons_Master_Component_C|GetDamageType _myweapon) (Variables|/Game/Blueprints/Weapons/Components/BP_Weapons_Master_Component.BP_Weapons_Master_Component_C|GetDamageResponses _myweapon) true false (Variables|/Game/Blueprints/Weapons/Components/BP_Weapons_Master_Component.BP_Weapons_Master_Component_C|GetShould%20Cam%20Follow%20on%20Death? _myweapon) (Variables|/Game/Blueprints/Weapons/Components/BP_Weapons_Master_Component.BP_Weapons_Master_Component_C|GetShould%20Impulse%20on%20Death? _myweapon)) _impactnormal _impactpoint (Variables|Default|GetInstigatingPlayer)))
      (if _wasdamaged_
        (Default|HitsUpdate (Variables|Default|GetInstigatingPlayer)))
      (CallFunction|DestroyProjectile))))

(fn ConstructionScript)