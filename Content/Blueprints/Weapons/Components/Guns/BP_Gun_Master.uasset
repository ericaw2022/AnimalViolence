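; Base gun component that fires either a projectile actor or an attached particle stream from the player mesh's socket.
; Particle shots go through server RPC to multicast, spawning the effect and setting timers for sphere traces along it that send damage messages.
; Traces run directly for a locally controlled authority or via ROS_Trace on remotes.
; Acid guns repeat the multicast in a delayed burst; StopShoot deactivates particles and clears timers.
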(event Custom|ParticleShootTrace
  (Networking|SwitchHasAuthority
    (:Authority
      (if (Pawn|IsLocallyControlled (Variables|Default|GetInstigatingPlayer))
        (bind _returnvalue (Utilities|Time|SetTimerbyEvent (delegate Custom|Trace) (Variables|Default|GetParticleDMGTime)))
        (Variables|Default|SetLocal _returnvalue)))
    (:Remote
      (bind _returnvalue_2 (Utilities|Time|SetTimerbyEvent (delegate Custom|ROS_Trace) (Variables|Default|GetParticleDMGTime)))
      (Variables|Default|SetRemote _returnvalue_2))))

(event Custom|ROS_Trace
  (bind _self self)
  (bind _activeparticles (Variables|Default|GetActiveParticles)
    (:then
      (bind (_outhit _returnvalue) (Collision|SphereTraceForObjects (Transformation|GetWorldLocation _activeparticles) (+ (Transformation|GetWorldLocation _activeparticles) (* (Math|Vector|GetForwardVector _activeparticles) (Variables|Default|GetProjectileDistance self))) 8e+01 (Utilities|Array|MakeArray "ObjectTypeQuery3" "ObjectTypeQuery2") false (Utilities|Array|MakeArray (Variables|Default|GetInstigatingPlayer)) "ForDuration" false))
      (if _returnvalue
        (Class|BPIDamagable|TakeDamage(Message) (.HitActor (Collision|BreakHitResult _outhit)) (Utilities|Struct|MakeS_DamageInfo (Variables|/Game/Blueprints/Weapons/Components/BP_Weapons_Master_Component.BP_Weapons_Master_Component_C|GetDamageAmount _self) (Variables|/Game/Blueprints/Weapons/Components/BP_Weapons_Master_Component.BP_Weapons_Master_Component_C|GetDamageType _self) (Variables|/Game/Blueprints/Weapons/Components/BP_Weapons_Master_Component.BP_Weapons_Master_Component_C|GetDamageResponses _self) false false (Variables|/Game/Blueprints/Weapons/Components/BP_Weapons_Master_Component.BP_Weapons_Master_Component_C|GetShould%20Cam%20Follow%20on%20Death? _self) (Variables|/Game/Blueprints/Weapons/Components/BP_Weapons_Master_Component.BP_Weapons_Master_Component_C|GetShould%20Impulse%20on%20Death? _self)) (.ImpactNormal (Collision|BreakHitResult _outhit)) (.ImpactPoint (Collision|BreakHitResult _outhit)) (Variables|Default|GetInstigatingPlayer))))
    (:else)))

(event Custom|MC_ShootParticles
  (bind _projectilesocketname (Variables|Default|GetProjectileSocketName))
  (bind _instigatingplayer (Variables|Default|GetInstigatingPlayer))
  (bind _mesh (Variables|/Script/Engine.Character|GetMesh _instigatingplayer))
  (if (Variables|Default|GetUsesParticles?)
    (bind _shootparticles__if_any_ (Variables|Default|GetShootParticles%20%28if%20any%29)
      (:then
        (bind _returnvalue (Niagara|SpawnSystemAttached _shootparticles__if_any_ self _projectilesocketname (Transformation|GetSocketLocation _mesh _projectilesocketname) (Transformation|GetSocketRotation _mesh _projectilesocketname) "KeepWorldPosition" true))
        (Variables|Default|SetActiveParticles _returnvalue)
        (CallFunction|ParticleShootTrace))
      (:else))))

(event Custom|Trace
  (bind _self self)
  (bind _activeparticles (Variables|Default|GetActiveParticles)
    (:then
      (bind (_outhit _returnvalue) (Collision|SphereTraceForObjects (Transformation|GetWorldLocation _activeparticles) (+ (Transformation|GetWorldLocation _activeparticles) (* (Math|Vector|GetForwardVector _activeparticles) (Variables|Default|GetProjectileDistance self))) 8e+01 (Utilities|Array|MakeArray "ObjectTypeQuery3" "ObjectTypeQuery2") false (Utilities|Array|MakeArray (Variables|Default|GetInstigatingPlayer)) "ForDuration" false))
      (if _returnvalue
        (Class|BPIDamagable|TakeDamage(Message) (.HitActor (Collision|BreakHitResult _outhit)) (Utilities|Struct|MakeS_DamageInfo (Variables|/Game/Blueprints/Weapons/Components/BP_Weapons_Master_Component.BP_Weapons_Master_Component_C|GetDamageAmount _self) (Variables|/Game/Blueprints/Weapons/Components/BP_Weapons_Master_Component.BP_Weapons_Master_Component_C|GetDamageType _self) (Variables|/Game/Blueprints/Weapons/Components/BP_Weapons_Master_Component.BP_Weapons_Master_Component_C|GetDamageResponses _self) false false (Variables|/Game/Blueprints/Weapons/Components/BP_Weapons_Master_Component.BP_Weapons_Master_Component_C|GetShould%20Cam%20Follow%20on%20Death? _self) (Variables|/Game/Blueprints/Weapons/Components/BP_Weapons_Master_Component.BP_Weapons_Master_Component_C|GetShould%20Impulse%20on%20Death? _self)) (.ImpactNormal (Collision|BreakHitResult _outhit)) (.ImpactPoint (Collision|BreakHitResult _outhit)) (Variables|Default|GetInstigatingPlayer))))
    (:else)))

(event Custom|ROS_ShootParticles
  (CallFunction|MCShootParticles)
  (if (Variables|Default|GetIsAcid?)
    (Utilities|Firing)))

(event Custom|ROS_StopShoot
  (CallFunction|MCStopShoot))

(event Custom|MC_StopShoot
  (if (Variables|Default|GetUsesParticles?)
    (bind _activeparticles (Variables|Default|GetActiveParticles)
      (:then
        (Components|Activation|Deactivate _activeparticles)
        (Utilities|Time|ClearandInvalidateTimerbyHandle (Variables|Default|GetLocal))
        (Utilities|Time|ClearandInvalidateTimerbyHandle (Variables|Default|GetRemote)))
      (:else))))

(event EventBeginPlay
  (|CallParentFunction) ; This node is disabled and will not be called.\nDrag off pins to build functionality.
)

(event EventTick
  (params (DeltaSeconds :type Float%20%28single-precision%29))
  (|CallParentFunction DeltaSeconds))

(event EventStopShoot
  (CallFunction|ROSStopShoot))

(event EventInstigPlayer
  (params (Instigator :type BP%20Combat%20Character%20Object%20Reference))
  (Variables|Default|SetInstigatingPlayer Instigator))

(fn Shoot
  (params (Instigator :type BP%20Combat%20Character%20Object%20Reference))
  (bind _instigatingplayer (Variables|Default|GetInstigatingPlayer))
  (bind _projectilesocketname (Variables|Default|GetProjectileSocketName))
  (bind _mesh (Variables|/Script/Engine.Character|GetMesh _instigatingplayer))
  (if (Variables|Default|GetUsesProjectile?)
    (bind _projectileactor__if_any_ (Variables|Default|GetProjectileActor%20%28if%20any%29)
      (:then
        (Game|SpawnActorfromClass _projectileactor__if_any_ (Math|Transform|MakeTransform (Transformation|GetSocketLocation _mesh _projectilesocketname) (Transformation|GetSocketRotation _mesh _projectilesocketname) "1.000000,1.000000,1.000000") "Undefined" "MultiplyWithRoot" 0 self (Variables|Default|GetInstigatingPlayer) 0))
      (:else
        _))
    (return)
    (elif (Variables|Default|GetUsesParticles?)
      (CallFunction|ROSShootParticles)
      (return)
      (else
        (return)))))