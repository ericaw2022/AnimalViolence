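; Master Blueprint for a networked weapon pickup that gives its configured weapon to the character who interacts with it, then destroys itself.
; The authority runs physics, forces periodic net updates against position desync and optionally destroys the pickup after a decay timer, while remotes keep physics off.
; Interact routes through ROS_SpawnWeapon to the character's SpawnWeapon.
; Radius overlaps by player character 0 toggle custom depth for an outline.
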(event OnComponentBeginOverlap(PickUpRadius)
  (params (OverlappedComponent :type Primitive%20Component%20Object%20Reference) (OtherActor :type Actor%20Object%20Reference) (OtherComp :type Primitive%20Component%20Object%20Reference) (OtherBodyIndex :type Integer) (bFromSweep :type Boolean) (SweepResult :type Hit%20Result%20Structure%20%28by%20ref%29))
  ;[0.15 0.15 0.15 0.5] outlines
  (if (== OtherActor (Game|GetPlayerCharacter 0))
    (Rendering|SetRenderCustomDepth (Variables|Default|GetPickUp%20Object) true)))

(event OnComponentEndOverlap(PickUpRadius)
  (params (OverlappedComponent :type Primitive%20Component%20Object%20Reference) (OtherActor :type Actor%20Object%20Reference) (OtherComp :type Primitive%20Component%20Object%20Reference) (OtherBodyIndex :type Integer))
  ;[0.15 0.15 0.15 0.5] outlines
  (if (== OtherActor (Game|GetPlayerCharacter 0))
    (Rendering|SetRenderCustomDepth (Variables|Default|GetPickUp%20Object) false)))

(event Custom|ROS_SpawnWeapon
  (params (Target :type BP%20Combat%20Character%20Object%20Reference) (WeaponToSpawn :type BP%20Weapons%20Master%20Component%20Class%20Reference))
  ;[0.15 0.15 0.15 0.5] interact
  (Default|SpawnWeapon Target WeaponToSpawn)
  (Actor|DestroyActor))

(event Custom|SelfDestroy
  ;[0.15 0.15 0.15 0.5] self destroy
  (Actor|DestroyActor))

(event Custom|CheckPositionDesync
  (Networking|ForceNetUpdate))

(event EventBeginPlay
  ;[0.15 0.15 0.15 0.5] self destroy
  (Networking|SwitchHasAuthority
    (:Authority
      (Physics|SetSimulatePhysics (Variables|Default|GetPickUp%20Object) true)
      (Utilities|Time|SetTimerbyEvent (delegate Custom|CheckPositionDesync) 0.5 true)
      (if (Variables|Default|GetDecay?)
        (Utilities|Time|SetTimerbyEvent (delegate Custom|SelfDestroy) (Variables|Default|GetTimeUntilDecay))))
    (:Remote
      (Physics|SetSimulatePhysics (Variables|Default|GetPickUp%20Object) false))))

(event EventInteract
  (params (CharacterPickingUp :type BP%20Combat%20Character%20Object%20Reference))
  ;[0.15 0.15 0.15 0.5] interact
  (CallFunction|ROSSpawnWeapon CharacterPickingUp (Variables|Default|GetWeaponToSpawn)))

(fn ConstructionScript)