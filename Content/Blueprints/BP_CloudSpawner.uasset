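; Cloud spawner Blueprint that scatters NS_Clouds Niagara effects through a sky volume when play begins.
; A single BeginPlay loop, driven by NumOfCloudstoSpawn, spawns each system at a random point within the SkyVolume component's bounds.
; Each spawn gets a random roll over a full turn, while yaw uses a plain RandomFloat, so it varies by at most one degree.
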(event EventBeginPlay
  (bind _skyvolume (Variables|Default|GetSkyVolume))
  (bind (_origin _boxextent) (Collision|GetComponentBounds _skyvolume))
  (for _index (range 0 (Variables|Default|GetNumOfCloudstoSpawn))
    (Niagara|SpawnSystematLocation "/Game/VFX/Clouds/NS_Clouds.NS_Clouds" (Math|Vector|MakeVector (Math|Random|RandomFloatinRange (- (.x _origin) (.x _boxextent)) (+ (.x _origin) (.x _boxextent))) (Math|Random|RandomFloatinRange (- (.y _origin) (.y _boxextent)) (+ (.y _origin) (.y _boxextent))) (Math|Random|RandomFloatinRange (- (.z _origin) (.z _boxextent)) (+ (.z _origin) (.z _boxextent)))) (Math|Rotator|MakeRotator (Math|Random|RandomFloatinRange 0.0 3.6e+02) 0.0 (Math|Random|RandomFloat)))))

(fn ConstructionScript)