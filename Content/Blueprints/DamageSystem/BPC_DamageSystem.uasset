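; Actor component that handles health, healing and damage intake for the actor that owns it.
; TakeDamage reads a DamageInfo and passes through a CanBeDamaged gate that rejects dead targets and invincible ones unless overridden.
; Damage fires OnDeath at zero health, or OnDamageResponse when the target is interruptible or the hit forces interruption.
; Heal clamps health to MaxHealth and only works while alive.
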(event EventBeginPlay)

(event EventTick
  (params (DeltaSeconds :type Float%20%28single-precision%29)))

(fn Heal
  (params (Amount :type Float%20%28double-precision%29))
  (if (not (Variables|Default|GetIsDead?))
    (bind _output_get (Variables|Default|SetHealth (Math|Float|Clamp(Float) (+ Amount (Variables|Default|GetHealth)) 0.0 (Variables|Default|GetMaxHealth))))
    (return _output_get)))

(fn TakeDamage
  (params (DamageInfo :type S%20Damage%20Info%20Structure) (NormalLocation :type Vector) (ActorLocation :type Vector))
  (bind (_amount _damagetype _damageresponse _shoulddamageinvincible_ _shouldforceinterrupt_ _shouldcamfollowondeath_ _shouldimpulseondeath_) (Utilities|Struct|BreakS_DamageInfo DamageInfo))
  (Utilities|CanbeDamaged? _shoulddamageinvincible_
    (:DoDamage
      (bind _output_get (Variables|Default|SetHealth (- (Variables|Default|GetHealth) _amount)))
      (if (<= _output_get 0.0)
        (Variables|Default|SetIsDead? true)
        (Default|CallOnDeath _shouldcamfollowondeath_ _shouldimpulseondeath_)
        (return true)
        (elif (or (Variables|Default|GetIsInterruptible?) _shouldforceinterrupt_)
          (Default|CallOnDamageResponse _damageresponse NormalLocation ActorLocation)
          (return true))))
    (:NoDamage
      (return false))))