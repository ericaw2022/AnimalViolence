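; BP_LobbySign is a sign actor, named for the lobby, that flips between two sign meshes and moves vertically.
; Switch spins the main mesh toward 90 yaw on a timeline, toggles visibility on both meshes, then calls Spin2 to continue toward 270.
; BeginMove uses a separate timeline to lerp only the height toward BeginLOC's Z.
; Each lerp starts from the current transform every update, easing toward its target.
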(event Custom|Spin2
  (bind _spin (Timeline|Timeline PlayFromStart)
    (:Update
      (Transformation|SetWorldRotation (Variables|Debug|GetStaticMeshComponent) (Math|Rotator|Lerp(Rotator) (Transformation|GetWorldRotation (Variables|Debug|GetStaticMeshComponent)) "0.000000,270.000000,0.000000" _spin) false false))))

(event EventBeginMove
  (bind _staticmeshcomponent (Variables|Debug|GetStaticMeshComponent))
  (bind _returnvalue (Transformation|GetWorldLocation _staticmeshcomponent))
  (bind _move (Timeline|Move Play)
    (:Update
      (Transformation|SetWorldLocation (Variables|Debug|GetStaticMeshComponent) (Math|Vector|Lerp(Vector) (Math|Vector|MakeVector (.x _returnvalue) (.y _returnvalue) (.z _returnvalue)) (Math|Vector|MakeVector (.x _returnvalue) (.y _returnvalue) (.z (Variables|Default|GetBeginLOC))) _move) false false))))

(event EventSwitch
  (bind _spin (Timeline|Spin Play)
    (:Update
      (Transformation|SetWorldRotation (Variables|Debug|GetStaticMeshComponent) (Math|Rotator|Lerp(Rotator) (Transformation|GetWorldRotation (Variables|Debug|GetStaticMeshComponent)) "0.000000,90.000000,0.000000" _spin) false false))
    (:Finished
      (Rendering|ToggleVisibility (Variables|Debug|GetStaticMeshComponent) false)
      (Rendering|ToggleVisibility (Variables|Default|GetSM_Sign2) false)
      (CallFunction|Spin2))))

(fn ConstructionScript)