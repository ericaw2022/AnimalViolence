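; BP_TrailerCharacter2 is a character Blueprint, apparently for a trailer, that cycles its skeletal mesh through three animal models on a fixed timeline.
; BeginPlay starts a timer that swaps the mesh to Cat after a short delay.
; Each swap event then schedules the next through another event-bound timer, changing to Dog and finally Bunny, where the one-shot chain stops.
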(event Custom|CustomEvent_1
  (Components|SkeletalMesh|SetSkeletalMeshAsset (Variables|Default|GetSkeletalMesh) "/Game/Animals/Bunny/Bunny.Bunny"))

(event Custom|Change
  (Components|SkeletalMesh|SetSkeletalMeshAsset (Variables|Default|GetSkeletalMesh) "/Game/Animals/Cat/Cat.Cat")
  (Utilities|Time|SetTimerbyEvent (delegate Custom|CustomEvent) 1.0))

(event Custom|CustomEvent
  (Components|SkeletalMesh|SetSkeletalMeshAsset (Variables|Default|GetSkeletalMesh) "/Game/Animals/Dog/Dog.Dog")
  (Utilities|Time|SetTimerbyEvent (delegate Custom|CustomEvent_1) 1.0))

(event EventBeginPlay
  (Utilities|Time|SetTimerbyEvent (delegate Custom|Change) 3.0))

(fn ConstructionScript)