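; BP_PlayerState is a player state Blueprint that records a player's combat stats and round wins.
; Custom events increment deaths, kills, hits dealt, blood lost and wins, and set flags for death and round victory.
; Kill, hit and blood updates stop once the player is dead, while bleeding starts a looping one-second timer that keeps adding blood loss.
; Wins has a RepNotify function, currently empty.
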(event Custom|I%20died
  (Math|Integer|IncrementInt (Variables|Default|GetDeaths)
    (:%20%20
      (Variables|Default|SetAmIDead? true))))

(event Custom|I%20killed
  (if (not (Variables|Default|GetAmIDead?))
    (Math|Integer|IncrementInt (Variables|Default|GetKills))))

(event Custom|I'm%20bleeding
  (if (not (Variables|Default|GetAmIDead?))
    (Utilities|Time|SetTimerbyEvent (delegate Custom|TrackBloodLoss) 1.0 true)))

(event Custom|I%20got%20hit
  (if (not (Variables|Default|GetAmIDead?))
    (Math|Integer|IncrementInt (Variables|Default|GetLostBlood))))

(event Custom|TrackBloodLoss
  (if (not (Variables|Default|GetAmIDead?))
    (Math|Integer|IncrementInt (Variables|Default|GetLostBlood))))

(event Custom|Ihitsomeone
  (if (not (Variables|Default|GetAmIDead?))
    (Math|Integer|IncrementInt (Variables|Default|GetHitsDealt))))

(event Custom|IWon
  (Variables|Default|SetDidIWinRound? true)
  (Math|Integer|IncrementInt (Variables|Default|GetWins)))

(event EventBeginPlay)

(event EventTick
  (params (DeltaSeconds :type Float%20%28single-precision%29)))

(fn ConstructionScript)

(fn OnRepWins)