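; BP_LobbyCam_LobbyMenu2 is a lobby camera Blueprint that adjusts its Nail3 and Nail4 components for clients.
; On BeginPlay, it runs the parent logic, then loops over every BP_CombatPlayerController.
; For each controller without authority, it toggles the visibility of both nails without propagating to children, so repeated matches flip them again.
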(event EventBeginPlay
  (|CallParentFunction)
  (bind _outactors (Actor|GetAllActorsOfClass "/Game/Variant_Combat/Blueprints/BP_CombatPlayerController.BP_CombatPlayerController_C"))
  (for _array_element _outactors
    (if (not (Ability|HasAuthority _array_element))
      (Rendering|ToggleVisibility (Variables|Default|GetNail3) false)
      (Rendering|ToggleVisibility (Variables|Default|GetNail4) false))))

(event Collision|EventActorBeginOverlap
  (params (OtherActor :type Actor%20Object%20Reference)))

(event EventTick
  (params (DeltaSeconds :type Float%20%28single-precision%29)))

(fn ConstructionScript
  (|CallParentFunction))