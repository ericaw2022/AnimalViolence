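; BP_LobbyCam_MainMenu is the main menu lobby camera actor, linking 3D Settings and Find buttons to transitions into other menus.
; On BeginPlay it casts the widgets of its two widget components and binds each button's TransitionToLinkedMenu event to Transition.
; Transition validates the menu index, then passes that LinkedMenus entry to TransitionTo.
; A failed Settings cast also leaves the Find button unbound.
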(event Custom|Transition
  (params (MenuInt :type Integer))
  (bind _linkedmenus (Variables|Default|GetLinkedMenus))
  (if (Utilities|Array|IsValidIndex _linkedmenus MenuInt)
    (CallFunction|Transitionto (Utilities|Array|Get(acopy) _linkedmenus MenuInt))))

(event EventBeginPlay
  (bind _aswb_3d_settings_button (Utilities|Casting|CastToWB_3D_SettingsButton (UserInterface|GetWidget (Variables|Default|GetSettingsWidget))))
  (EventDispatchers|BindEventtoTransitiontoLinkedMenu _aswb_3d_settings_button (delegate Custom|Transition))
  (bind _aswb_3d_find_button (Utilities|Casting|CastToWB_3D_FindButton (UserInterface|GetWidget (Variables|Default|GetFindWidget))))
  (EventDispatchers|BindEventtoTransitiontoLinkedMenu _aswb_3d_find_button (delegate Custom|Transition)))

(event Collision|EventActorBeginOverlap
  (params (OtherActor :type Actor%20Object%20Reference))
  (|CallParentFunction OtherActor) ; This node is disabled and will not be called.\nDrag off pins to build functionality.
)

(event EventTick
  (params (DeltaSeconds :type Float%20%28single-precision%29))
  (|CallParentFunction DeltaSeconds) ; This node is disabled and will not be called.\nDrag off pins to build functionality.
)

(fn ConstructionScript
  (|CallParentFunction))