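; BP_LobbyCam_FindMenu is a lobby camera Blueprint for the find menu, handling transitions back to linked menus.
; On BeginPlay it casts its BackWidget's widget to WB_3D_BackFindButton and binds that button's transition event.
; When the event fires, it validates the menu index against LinkedMenus and calls TransitionTo on that entry.
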(event Custom|TransitionBack
  (params (MenuInt :type Integer))
  (bind _linkedmenus (Variables|Default|GetLinkedMenus))
  (if (Utilities|Array|IsValidIndex _linkedmenus MenuInt)
    (CallFunction|Transitionto (Utilities|Array|Get(acopy) _linkedmenus MenuInt))))

(event EventBeginPlay
  (|CallParentFunction)
  (bind _aswb_3d_back_find_button (Utilities|Casting|CastToWB_3D_BackFindButton (UserInterface|GetWidget (Variables|Default|GetBackWidget))))
  (EventDispatchers|BindEventtoTransitiontoLinkedMenu _aswb_3d_back_find_button (delegate Custom|TransitionBack)))

(fn ConstructionScript
  (|CallParentFunction))