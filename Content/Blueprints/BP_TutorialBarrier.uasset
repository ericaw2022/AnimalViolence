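; BP_TutorialBarrier is a tutorial barrier that slides its Object component to a set location when triggered.
; Trigger notifies the tutorial HUD widgets and, inside that loop, plays the Move timeline, lerping from the starting relative location to SelectLOC at a configurable rate.
; When the move finishes, it fires the first valid of three spawners in priority order, with the second also starting the Car.
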(event EventBeginPlay
  (Variables|Default|SetEndLOC (Variables|Default|GetSelectLOC))
  (Variables|Default|SetStartLOC (Variables|/Script/Engine.SceneComponent|GetRelativeLocation (Variables|Default|GetObject)))
  (Components|Timeline|SetPlayRate (Variables|Default|GetMove) (Variables|Default|GetTimeRate)))

(event EventTrigger
  (bind _foundwidgets (Widget|GetAllWidgetsOfClass "/Game/UI/WB_HUD_Tutorial.WB_HUD_Tutorial_C" true))
  (for _array_element _foundwidgets
    (Default|Triggered _array_element)
    (bind _move (Timeline|Move Play)
      (:Update
        (Transformation|SetRelativeLocation (Variables|Default|GetObject) (Math|Vector|Lerp(Vector) (Variables|Default|GetStartLOC) (Variables|Default|GetEndLOC) _move) false false))
      (:Finished
        (bind _spawner (Variables|Default|GetSpawner)
          (:then
            (Default|Spawn _spawner))
          (:else
            (bind _2ndspawner (Variables|Default|Get2ndSpawner)
              (:then
                (Default|Spawn _2ndspawner)
                (Default|StartCar (Variables|Default|GetCar)))
              (:else
                (bind _3rdspawner (Variables|Default|Get3rdSpawner)
                  (:then
                    (Default|Spawn _3rdspawner))
                  (:else))))))))))

(fn ConstructionScript)