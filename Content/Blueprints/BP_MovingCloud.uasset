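; BP_MovingCloud is a moving platform that shuttles its Object component back and forth between its starting relative location and a configured target, SelectLOC.
; On BeginPlay it stores both endpoints and sets the Move timeline's play rate from TimeRate.
; The timeline lerps the relative location without sweep.
; On finish, it waits DelayBeforeMove and calls MovePlatform again, where a FlipFlop alternates forward and reverse playback for an endless loop.
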(event Custom|MovePlatform
  (Utilities|FlowControl|FlipFlop
    (:A
      (bind _move (Timeline|Move PlayFromStart)
        (:Update
          (Transformation|SetRelativeLocation (Variables|Default|GetObject) (Math|Vector|Lerp(Vector) (Variables|Default|GetStartLOC) (Variables|Default|GetEndLOC) _move) false false))
        (:Finished
          (Utilities|FlowControl|Delay (Variables|Default|GetDelayBeforeMove))
          (CallFunction|MovePlatform))))
    (:B
      (Timeline|Move ReverseFromEnd))))

(event EventBeginPlay
  (Variables|Default|SetEndLOC (Variables|Default|GetSelectLOC))
  (Variables|Default|SetStartLOC (Variables|/Script/Engine.SceneComponent|GetRelativeLocation (Variables|Default|GetObject)))
  (Components|Timeline|SetPlayRate (Variables|Default|GetMove) (Variables|Default|GetTimeRate))
  (CallFunction|MovePlatform))

(fn ConstructionScript)