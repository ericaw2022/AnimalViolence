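; Fixed camera actor that switches the player's view to itself when the player character enters its trigger box.
; BeginPlay caches the player as a BP_CombatCharacter.
; On box overlap by the player, it blends the controller's view target to this actor using configurable time and blend function, sets the character's DisableCamera flag and removes all widgets from the screen.
; No exit handling restores the previous view.
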(event OnComponentBeginOverlap(Box)
  (params (OverlappedComponent :type Primitive%20Component%20Object%20Reference) (OtherActor :type Actor%20Object%20Reference) (OtherComp :type Primitive%20Component%20Object%20Reference) (OtherBodyIndex :type Integer) (bFromSweep :type Boolean) (SweepResult :type Hit%20Result%20Structure%20%28by%20ref%29))
  (if (== OtherActor (Game|GetPlayerCharacter 0))
    (CallFunction|OnFixedCamOverlap)
    (Variables|/Game/Variant_Combat/Blueprints/BP_CombatCharacter.BP_CombatCharacter_C|SetDisableCamera (Variables|Default|GetChar) true)
    (Viewport|RemoveAllWidgets)))

(event EventBeginPlay
  (bind _asbp_combat_character (Utilities|Casting|CastToBP_CombatCharacter (Game|GetPlayerCharacter 0)))
  (Variables|Default|SetChar _asbp_combat_character))

(fn ConstructionScript)

(fn OnFixedCamOverlap
  (Game|Player|SetViewTargetwithBlend (Game|GetPlayerController 0) self (Variables|Default|GetBlend%20Time) (Variables|Default|GetBlend%20Func) 0.0 false))