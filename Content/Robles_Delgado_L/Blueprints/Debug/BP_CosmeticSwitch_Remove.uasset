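; Debug cosmetic switch actor that removes hats from a BP_CombatCharacter overlapping its box, displaying TargetMesh on BeginPlay.
; On overlap it detaches the character mesh's children on Hat_Socket, keeping world transform.
; It then tries teleporting its own mesh to a hat switch's OGSpawn, but casts the overlapping character to BP_CosmeticSwitch_Hat, so that step likely never runs.
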(event OnComponentBeginOverlap(Box1)
  (params (OverlappedComponent :type Primitive%20Component%20Object%20Reference) (OtherActor :type Actor%20Object%20Reference) (OtherComp :type Primitive%20Component%20Object%20Reference) (OtherBodyIndex :type Integer) (bFromSweep :type Boolean) (SweepResult :type Hit%20Result%20Structure%20%28by%20ref%29))
  (bind _asbp_combat_character (Utilities|Casting|CastToBP_CombatCharacter OtherActor))
  (for _array_element (Components|GetChildrenComponents (Variables|/Script/Engine.Character|GetMesh _asbp_combat_character) false)
    (if (== (Transformation|GetAttachSocketName _array_element) "Hat_Socket")
      (Transformation|DetachFromComponent _array_element "KeepWorld" "KeepWorld" "KeepWorld" true)
      (bind _asbp_cosmetic_switch_hat (Utilities|Casting|CastToBP_CosmeticSwitch_Hat OtherActor))
      (Transformation|SetWorldTransform (Variables|Default|GetTheMesh) (Variables|/Game/Robles_Delgado_L/Blueprints/Debug/BP_CosmeticSwitch_Hat.BP_CosmeticSwitch_Hat_C|GetOGSpawn _asbp_cosmetic_switch_hat) false true))))

(event EventBeginPlay
  (Utilities|Casting|CastToBP_CombatCharacter (Game|GetPlayerCharacter 0))
  (Components|StaticMesh|SetStaticMesh (Variables|Default|GetTheMesh) (Variables|Default|GetTargetMesh)))

(event Collision|EventActorBeginOverlap
  (params (OtherActor :type Actor%20Object%20Reference)))

(event EventTick
  (params (DeltaSeconds :type Float%20%28single-precision%29)))

(fn ConstructionScript)

(fn OnRepTargetMesh)