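; BP_CosmeticSwitch_Hat is a debug-folder pickup actor that puts a hat mesh on the player character.
; BeginPlay applies TargetMesh to TheMesh and saves its world transform, provided the player is a BP_CombatCharacter.
; Overlapping Box1 snaps TheMesh itself onto that character's Hat_Socket.
; Unconnected launch and car-hit death nodes never run, and the TargetMesh OnRep is empty.
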(event OnComponentBeginOverlap(Box1)
  (params (OverlappedComponent :type Primitive%20Component%20Object%20Reference) (OtherActor :type Actor%20Object%20Reference) (OtherComp :type Primitive%20Component%20Object%20Reference) (OtherBodyIndex :type Integer) (bFromSweep :type Boolean) (SweepResult :type Hit%20Result%20Structure%20%28by%20ref%29))
  (bind _asbp_combat_character (Utilities|Casting|CastToBP_CombatCharacter OtherActor))
  (Transformation|AttachComponentToComponent (Variables|Default|GetTheMesh) (Variables|/Script/Engine.Character|GetMesh _asbp_combat_character) "Hat_Socket" "SnapToTarget" "SnapToTarget" "SnapToTarget" true))

(event EventBeginPlay
  (Utilities|Casting|CastToBP_CombatCharacter (Game|GetPlayerCharacter 0))
  (Components|StaticMesh|SetStaticMesh (Variables|Default|GetTheMesh) (Variables|Default|GetTargetMesh))
  (Variables|Default|SetOGSpawn (Transformation|GetWorldTransform (Variables|Default|GetTheMesh))))

(event Collision|EventActorBeginOverlap
  (params (OtherActor :type Actor%20Object%20Reference)))

(event EventTick
  (params (DeltaSeconds :type Float%20%28single-precision%29)))

(fn ConstructionScript)

(fn OnRepTargetMesh)