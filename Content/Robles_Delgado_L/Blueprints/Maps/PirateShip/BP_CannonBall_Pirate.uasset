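; Cannonball projectile for the PirateShip map that damages what it hits.
; On BeginPlay it plays an attached whistle sound with projectile attenuation, stopping when the ball is destroyed.
; Hits are handled on the authority only, through a DoOnce gate that a one-second timer resets.
; When the Projectile component is the one hit, it sends fixed damage to the other actor via TakeDamageMessage and destroys itself.
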(event Custom|OpenGate
  (Utilities|FlowControl|DoOnce false) ; enters at Reset
)

(event EventBeginPlay
  (Audio|SpawnSoundAttached "/Game/Robles_Delgado_L/Sounds/Weapons/Samples/ShWeaponProjectileWhistle.ShWeaponProjectileWhistle" (Variables|Default|GetProjectile) "None" (Transformation|GetWorldLocation (Variables|Default|GetProjectile)) "0, 0, 0" "SnapToTarget" true 1.0 1.0 0.0 "/Game/Robles_Delgado_L/Sounds/SoundAttenuation_Projectile.SoundAttenuation_Projectile" 0))

(event Collision|EventActorBeginOverlap
  (params (OtherActor :type Actor%20Object%20Reference)))

(event EventTick
  (params (DeltaSeconds :type Float%20%28single-precision%29)))

(event Collision|EventHit
  (params (MyComp :type Primitive%20Component%20Object%20Reference) (Other :type Actor%20Object%20Reference) (OtherComp :type Primitive%20Component%20Object%20Reference) (bSelfMoved :type Boolean) (HitLocation :type Vector :default "0, 0, 0") (HitNormal :type Vector :default "0, 0, 0") (NormalImpulse :type Vector :default "0, 0, 0") (Hit :type Hit%20Result%20Structure%20%28by%20ref%29))
  (Networking|SwitchHasAuthority
    (:Authority
      (Utilities|FlowControl|DoOnce false
        (:Completed
          (Utilities|Time|SetTimerbyEvent (delegate Custom|OpenGate) 1.0)
          (if (== MyComp (Variables|Default|GetProjectile))
            (Class|BPIDamagable|TakeDamage(Message) Other (Utilities|Struct|MakeS_DamageInfo 5e+01 "NewEnumerator4" "NewEnumerator1" false false true true) HitNormal HitLocation)
            (Actor|DestroyActor)))))))

(fn ConstructionScript
  (|CallParentFunction))