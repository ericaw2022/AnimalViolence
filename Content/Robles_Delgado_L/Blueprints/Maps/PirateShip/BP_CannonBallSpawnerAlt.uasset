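; Pirate ship cannon spawner that fires scaled-up BP_CannonBall_PirateAlt actors from SpawnLocation with an attenuated shot sound.
; BeginPlay hides the preview, optionally the base mesh, then either fires once or starts a looping timer whose random interval is rolled only once.
; When ShouldFirstItemSpawn is set, it fires a single shot and never starts the timer.
; Spawns route through ROS_ events; the velocity-setting code is disconnected.
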(event Custom|ContinuousSpawn
  ;[0.15 0.15 0.15 0.5] Continuous
  (CallFunction|ROSContinuousSpawn))

(event Custom|SingularSpawn
  ;[0.15 0.15 0.15 0.5] Singular
  (CallFunction|ROSSingularSpawn))

(event Custom|ROS_ContinuousSpawn
  ;[0.15 0.15 0.15 0.5] Continuous
  (Audio|PlaySoundatLocation "/Game/Robles_Delgado_L/Sounds/Weapons/Cannon_Shoot.Cannon_Shoot" (Transformation|GetActorLocation) "0, 0, 0" 1.0 1.0 0.0 "/Game/Robles_Delgado_L/Sounds/SoundAttenuation_CannonPirate.SoundAttenuation_CannonPirate" 0 0 0)
  (Game|SpawnActorfromClass "/Game/Robles_Delgado_L/Blueprints/Maps/PirateShip/BP_CannonBall_PirateAlt.BP_CannonBall_PirateAlt_C" (Math|Transform|MakeTransform (Transformation|GetWorldLocation (Variables|Default|GetSpawnLocation)) "0, 0, 0" "5.000000,5.000000,5.000000") "Undefined" "MultiplyWithRoot" 0 0 0 0))

(event Custom|ROS_SingularSpawn
  ;[0.15 0.15 0.15 0.5] Singular
  (Audio|PlaySoundatLocation "/Game/Robles_Delgado_L/Sounds/Weapons/Cannon_Shoot.Cannon_Shoot" (Transformation|GetWorldLocation (Variables|Default|GetBaseObject)) "0, 0, 0" 1.0 1.0 0.0 "/Game/Robles_Delgado_L/Sounds/SoundAttenuation_CannonPirate.SoundAttenuation_CannonPirate" 0 0 0)
  (Game|SpawnActorfromClass "/Game/Robles_Delgado_L/Blueprints/Maps/PirateShip/BP_CannonBall_PirateAlt.BP_CannonBall_PirateAlt_C" (Math|Transform|MakeTransform (Transformation|GetWorldLocation (Variables|Default|GetSpawnLocation)) "0, 0, 0" "5.000000,5.000000,5.000000") "Undefined" "MultiplyWithRoot" 0 0 0 0))

(event EventBeginPlay
  (bind _baseobject (Variables|Default|GetBaseObject))
  ;[0.15 0.15 0.15 0.5] Init
  (if (Variables|Changable|GetShouldBaseObjectBeVisible?)
    _
    (else
      (Rendering|ToggleVisibility _baseobject false)
      (Collision|SetCollisionEnabled _baseobject "NoCollision")))
  (Rendering|ToggleVisibility (Variables|Default|GetPreviewAsset) false)
  (if (not (Variables|Changable|GetSpawnThroughoutGame?))
    (if (Variables|Changable|GetShouldFirstItemSpawn?)
      (CallFunction|SingularSpawn))
    (elif (Variables|Changable|GetShouldFirstItemSpawn?)
      (CallFunction|SingularSpawn)
      (else
        (Utilities|Time|SetTimerbyEvent (delegate Custom|ContinuousSpawn) (Math|Random|RandomFloatinRange (Variables|Changable|GetMinSpawnTime) (Variables|Changable|GetMaxSpawnTime)) true)))))

(fn ConstructionScript)