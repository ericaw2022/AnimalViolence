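; Tutorial traffic car that loops along a path and kills any combat enemy it overlaps, ignoring the player combat character.
; Once started, it waits, moves to its destination over a random duration, pauses randomly, recolors, teleports by an offset and repeats.
; Recoloring picks a random material from an array and sets ColorIndex, whose RepNotify applies the material to the car body.
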(event OnComponentBeginOverlap(Box)
  (params (OverlappedComponent :type Primitive%20Component%20Object%20Reference) (OtherActor :type Actor%20Object%20Reference) (OtherComp :type Primitive%20Component%20Object%20Reference) (OtherBodyIndex :type Integer) (bFromSweep :type Boolean) (SweepResult :type Hit%20Result%20Structure%20%28by%20ref%29))
  (Utilities|Casting|CastToBP_CombatCharacter OtherActor
    (:CastFailed
      (bind _asbp_combat_enemy (Utilities|Casting|CastToBP_CombatEnemy OtherActor))
      (Default|HandleDeath _asbp_combat_enemy))))

(event Custom|CarMovement
  (Utilities|FlowControl|Delay 2.0)
  (Components|MoveComponentTo (Variables|Transformation|GetRootComponent) (Variables|Default|GetCarDestination) (Transformation|GetActorRotation) false false (Math|Random|RandomFloatinRange (Variables|Default|GetCarSpeedMin) (Variables|Default|GetCarSpeedMax)) false :!label _label)
  (Utilities|FlowControl|Delay (Math|Random|RandomFloatinRange (Variables|Default|GetDelayMin) (Variables|Default|GetDelayMax)))
  (CallFunction|ColorRandomize)
  (Transformation|Teleport (+ (Transformation|GetActorLocation) (Variables|Default|GetTPLocation)) (Transformation|GetActorRotation))
  (goto _label))

(event Custom|StartCar
  (CallFunction|CarMovement))

(event Custom|ColorRandomize
  (bind _carcolorarray (Variables|Default|GetCarColorArray))
  (bind (_outitem _outindex) (Utilities|Array|Random _carcolorarray))
  (Variables|Default|SetRandomizedColor _outitem)
  (Variables|Default|SetColorIndex _outindex))

(event EventTick
  (params (DeltaSeconds :type Float%20%28single-precision%29)))

(fn ConstructionScript)

(fn OnRepCarColorArray)

(fn OnRepColorIndex
  (Rendering|Material|SetMaterial (Variables|Default|GetCarBody3D) 1 (Variables|Default|GetRandomizedColor)))