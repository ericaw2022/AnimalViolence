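; A test bomb projectile that, on first hit, flashes and ticks faster like a countdown, then destroys itself after about five seconds.
; A looping Activate event alternates red and black materials with a tick sound, while timed stages shorten the blink delay and switch the final sound.
; Shortly after BeginPlay it makes the player's combat character drop their weapon.
; Despite the SizeChangeTest name, nothing here changes size.
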(event OnComponentHit(Projectile)
  (params (HitComponent :type Primitive%20Component%20Object%20Reference) (OtherActor :type Actor%20Object%20Reference) (OtherComp :type Primitive%20Component%20Object%20Reference) (NormalImpulse :type Vector :default "0, 0, 0") (Hit :type Hit%20Result%20Structure%20%28by%20ref%29))
  (if (not (Variables|Default|GetHasStarted))
    (Variables|Default|SetSoundSpeed 0.5)
    (Variables|Default|SetHasStarted true)
    (CallFunction|Activate)
    (Utilities|FlowControl|Delay 1.0)
    (Variables|Default|SetSoundSpeed 0.4)
    (CallFunction|Activate)
    (Utilities|FlowControl|Delay 1.0)
    (Variables|Default|SetSoundSpeed 0.2)
    (CallFunction|Activate)
    (Utilities|FlowControl|Delay 1.0)
    (Variables|Default|SetSoundSpeed 0.08)
    (Variables|Default|SetSound "/Game/Robles_Delgado_L/Sounds/Weapons/BombTick2.BombTick2")
    (CallFunction|Activate)
    (Utilities|FlowControl|Delay 2.0)
    (Variables|Default|SetHasStarted false)
    (Actor|DestroyActor)))

(event Custom|ColorRed
  (bind _returnvalue (Rendering|Material|CreateDynamicMaterialInstance (Variables|Default|GetProjectile) 0 "/Game/Robles_Delgado_L/Models/Weapons/Bomb/BombRed.BombRed" "None" :!class /Script/Engine.PrimitiveComponent))
  (Rendering|Material|SetMaterial (Variables|Default|GetProjectile) 0 _returnvalue)
  (Audio|PlaySoundatLocation (Variables|Default|GetSound) (Transformation|GetWorldLocation (Variables|Default|GetProjectile)) "0, 0, 0" 1.0 1.0 0.0 0 0 0 0))

(event Custom|Activate
  (CallFunction|ColorRed :!label _label)
  (Utilities|FlowControl|Delay (Variables|Default|GetSoundSpeed))
  (CallFunction|ColorBlack)
  (Utilities|FlowControl|Delay (Variables|Default|GetSoundSpeed))
  (goto _label))

(event Custom|ColorBlack
  (bind _returnvalue (Rendering|Material|CreateDynamicMaterialInstance (Variables|Default|GetProjectile) 0 "/Game/Robles_Delgado_L/Models/Weapons/Bomb/Bomb1.Bomb1" "None" :!class /Script/Engine.PrimitiveComponent))
  (Rendering|Material|SetMaterial (Variables|Default|GetProjectile) 0 _returnvalue))

(event EventBeginPlay
  (bind _asbp_combat_character (Utilities|Casting|CastToBP_CombatCharacter (Game|GetPlayerCharacter 0)))
  (Utilities|FlowControl|Delay 0.02)
  (Default|DropWeaponSimple _asbp_combat_character))

(event Collision|EventActorBeginOverlap
  (params (OtherActor :type Actor%20Object%20Reference)))

(event EventTick
  (params (DeltaSeconds :type Float%20%28single-precision%29)))

(fn ConstructionScript
  (|CallParentFunction))