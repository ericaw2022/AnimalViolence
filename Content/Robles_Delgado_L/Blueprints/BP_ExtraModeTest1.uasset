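; Round-based multiplayer mode for animal combat that manages round start, round end and the overall winner.
; BeginPlay waits for ready players, restores looks and stats from GI_InfoStorage, then runs a countdown before Start enables input.
; When no players remain alive, it saves stats, shows scoreboards and server-travels to a random, non-repeating level.
; After the set number of rounds, most wins takes the game, with kills breaking ties.
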(event Custom|Check%20Remaining%20Players
  ;[0.15 0.15 0.15 0.5] Round Win Condition
  (Variables|Default|SetRemainingPlayers 0)
  (bind _asbp_game_state (Utilities|Casting|CastToBP_GameState (Game|GetGameState)))
  (for _array_element (Variables|/Script/Engine.GameStateBase|GetPlayerArray _asbp_game_state)
    (bind _asbp_player_state (Utilities|Casting|CastToBP_PlayerState _array_element))
    (if (not (Variables|/Game/Blueprints/GameInfo/BP_PlayerState.BP_PlayerState_C|GetAmIDead? _asbp_player_state))
      (Math|Integer|IncrementInt (Variables|Default|GetRemainingPlayers))))
  (CallFunction|EvaluatePlayerCount))

(event Custom|EvaluatePlayerCount
  ;[0.15 0.15 0.15 0.5] Round Win Condition
  (if (<= (Variables|Default|GetRemainingPlayers) 0)
    (for _array_element (Variables|/Script/Engine.GameStateBase|GetPlayerArray (Game|GetGameState))
      (bind _asbp_player_state (Utilities|Casting|CastToBP_PlayerState _array_element))
      (if (not (Variables|/Game/Blueprints/GameInfo/BP_PlayerState.BP_PlayerState_C|GetAmIDead? _asbp_player_state))
        (Default|IWon _asbp_player_state)))
    (CallFunction|RoundOver)))

(event Custom|RoundOver
  ;[0.15 0.15 0.15 0.5] Round Win Condition
  (bind _asgi_info_storage (Utilities|Casting|CastToGI_InfoStorage (Game|GetGameInstance)))
  (Default|SavePlayerInfo _asgi_info_storage)
  (Utilities|FlowControl|Delay (Variables|Default|GetDelayBeforeScoreboard))
  (for _array_element (Variables|/Script/Engine.GameStateBase|GetPlayerArray (Game|GetGameState))
    (bind _asbp_combat_player_controller (Utilities|Casting|CastToBP_CombatPlayerController (Components|GetOwner _array_element)))
    (Default|CallScoreboard _asbp_combat_player_controller))
  (Utilities|FlowControl|Delay (Variables|Default|GetDelayBeforeNextRound))
  (bind _wasgamewon_ (CallFunction|HasGameEnded?))
  (if (not _wasgamewon_)
    (CallFunction|SwitchRounds)))

(event Custom|TravelToSpecificLevel
  (params (LevelName :type Name))
  ;[0.15 0.15 0.15 0.5] GameOver
  (Utilities|FlowControl|Delay 1.0)
  (Development|ExecuteConsoleCommand (Utilities|String|Append "servertravel " (Utilities|String|ToString(Name) LevelName) "?listen") 0))

(event Custom|SwitchRounds
  ;[0.15 0.15 0.15 0.5] RoundSwitch
  (bind _asgi_info_storage (Utilities|Casting|CastToGI_InfoStorage (Game|GetGameInstance)))
  (Default|SaveCharacterModels _asgi_info_storage)
  (Default|SaveAnimalColors1 _asgi_info_storage)
  (Default|SaveAnimalColors2 _asgi_info_storage)
  (Utilities|FlowControl|Delay 1.0)
  (Networking|SwitchHasAuthority
    (:Authority
      (bind _asgi_info_storage_2 (Utilities|Casting|CastToGI_InfoStorage (Game|GetGameInstance)))
      (Variables|Default|SetCurrentLevel (.OutItem (Utilities|Array|Random (Variables|Default|GetLevel%20Names))))
      (if (not (== (Variables|Default|GetCurrentLevel) (Variables|/Game/Blueprints/GI_InfoStorage.GI_InfoStorage_C|GetLatestLevel _asgi_info_storage_2)))
        (bind _outactors (Actor|GetAllActorsOfClass "/Game/Variant_Combat/Blueprints/BP_CombatPlayerController.BP_CombatPlayerController_C"))
        (for _array_element _outactors
          (Default|RPCShowLoadingScreen _array_element (Variables|Default|GetCurrentLevel)))
        (Utilities|FlowControl|Delay 1.0)
        (Development|ExecuteConsoleCommand (Utilities|String|Append "servertravel " (Utilities|String|ToString(Name) (Variables|Default|GetCurrentLevel)) "?listen") 0)
        (bind _asgi_info_storage_3 (Utilities|Casting|CastToGI_InfoStorage (Game|GetGameInstance)))
        (Variables|/Game/Blueprints/GI_InfoStorage.GI_InfoStorage_C|SetLatestLevel _asgi_info_storage_3 (Variables|Default|GetCurrentLevel))
        (else
          (CallFunction|SwitchRounds))))))

(event EventBeginPlay
  ;[0.15 0.15 0.15 0.5] Start
  (bind _asgi_info_storage (Utilities|Casting|CastToGI_InfoStorage (Game|GetGameInstance)))
  (Default|SetGameInfo _asgi_info_storage)
  (for _array_element (Variables|/Script/Engine.GameStateBase|GetPlayerArray (Game|GetGameState))
    (bind _asbp_player_state (Utilities|Casting|CastToBP_PlayerState _array_element :!label _label))
    (if (not (Variables|/Game/Blueprints/GameInfo/BP_PlayerState.BP_PlayerState_C|GetPlayerReadyToStart? _asbp_player_state))
      (Utilities|FlowControl|Delay 0.5)
      (goto _label)))
  (Utilities|FlowControl|Delay 3.0)
  ;[0.15 0.15 0.15 0.5] Set prev info
  (Networking|SwitchHasAuthority
    (:Authority
      (bind _asbp_game_state (Utilities|Casting|CastToBP_GameState (Game|GetGameState)))
      (for _array_element_2 (Variables|/Script/Engine.GameStateBase|GetPlayerArray _asbp_game_state)
        (bind _asbp_player_state_2 (Utilities|Casting|CastToBP_PlayerState _array_element_2))
        (bind _asgi_info_storage_2 (Utilities|Casting|CastToGI_InfoStorage (Game|GetGameInstance)))
        (bind _asbp_combat_character (Utilities|Casting|CastToBP_CombatCharacter (PlayerState|GetPawn _asbp_player_state_2)))
        (Default|ServerSetMesh _asbp_combat_character (.Value (Utilities|Map|Find (Variables|/Game/Blueprints/GI_InfoStorage.GI_InfoStorage_C|GetAnimalNum _asgi_info_storage_2) (PlayerState|GetPlayerName _asbp_player_state_2))))
        (Default|ChangeColor1Server _asbp_combat_character (.Value (Utilities|Map|Find (Variables|/Game/Blueprints/GI_InfoStorage.GI_InfoStorage_C|GetAnimalColor1 _asgi_info_storage_2) (PlayerState|GetPlayerName _asbp_player_state_2))))
        (Variables|/Game/Blueprints/GameInfo/BP_PlayerState.BP_PlayerState_C|SetAnimalColorValue1 _asbp_player_state_2 (.Value (Utilities|Map|Find (Variables|/Game/Blueprints/GI_InfoStorage.GI_InfoStorage_C|GetAnimalColor1 _asgi_info_storage_2) (PlayerState|GetPlayerName _asbp_player_state_2))))
        (Default|ChangeColor2Server _asbp_combat_character (.Value (Utilities|Map|Find (Variables|/Game/Blueprints/GI_InfoStorage.GI_InfoStorage_C|GetAnimalColor2 _asgi_info_storage_2) (PlayerState|GetPlayerName _asbp_player_state_2))))
        (Variables|/Game/Blueprints/GameInfo/BP_PlayerState.BP_PlayerState_C|SetAnimalColorValue2 _asbp_player_state_2 (.Value (Utilities|Map|Find (Variables|/Game/Blueprints/GI_InfoStorage.GI_InfoStorage_C|GetAnimalColor2 _asgi_info_storage_2) (PlayerState|GetPlayerName _asbp_player_state_2))))
        (Variables|/Game/Blueprints/GameInfo/BP_PlayerState.BP_PlayerState_C|SetMeshChoiceNum _asbp_player_state_2 (.Value (Utilities|Map|Find (Variables|/Game/Blueprints/GI_InfoStorage.GI_InfoStorage_C|GetAnimalNum _asgi_info_storage_2) (PlayerState|GetPlayerName _asbp_player_state_2))))
        (Variables|/Game/Blueprints/GameInfo/BP_PlayerState.BP_PlayerState_C|SetWins _asbp_player_state_2 (.Wins (Utilities|Struct|BreakS_PlayerRankInfo (.Value (Utilities|Map|Find (Variables|/Game/Blueprints/GI_InfoStorage.GI_InfoStorage_C|GetPlayerInfo _asgi_info_storage_2) (PlayerState|GetPlayerName _asbp_player_state_2))))))
        (Variables|/Game/Blueprints/GameInfo/BP_PlayerState.BP_PlayerState_C|SetOverallKills _asbp_player_state_2 (.Kills (Utilities|Struct|BreakS_PlayerRankInfo (.Value (Utilities|Map|Find (Variables|/Game/Blueprints/GI_InfoStorage.GI_InfoStorage_C|GetPlayerInfo _asgi_info_storage_2) (PlayerState|GetPlayerName _asbp_player_state_2))))))
        (Utilities|FlowControl|Delay 0.0)
        (bind _outactors (Actor|GetAllActorsOfClass "/Game/Variant_Combat/Blueprints/BP_CombatPlayerController.BP_CombatPlayerController_C"))
        (for _array_element_3 _outactors
          (Default|StartHUDCountdown _array_element_3))
        (Utilities|Time|SetTimerbyFunctionName 0 "Start" (Variables|Default|GetStartTimer))))
    (:Remote
      (Utilities|FlowControl|Delay 0.0)
      (bind _outactors_2 (Actor|GetAllActorsOfClass "/Game/Variant_Combat/Blueprints/BP_CombatPlayerController.BP_CombatPlayerController_C"))
      (for _array_element_4 _outactors_2
        (Default|StartHUDCountdown _array_element_4))
      (Utilities|Time|SetTimerbyFunctionName 0 "Start" (Variables|Default|GetStartTimer)))))

(fn ConstructionScript)

(fn HasGameEnded?
  (bind _asgi_info_storage (Utilities|Casting|CastToGI_InfoStorage (Game|GetGameInstance)))
  (bind _result (Default|IncreaseRounds _asgi_info_storage))
  (if (>= _result (Variables|Default|GetRoundsNeededToEndGame))
    (bind _winner1 (CallFunction|WhoWontheGame?))
    (Variables|/Game/Blueprints/GameInfo/BP_PlayerState.BP_PlayerState_C|SetDidIWintheGame? _winner1 true)
    (bind _asgi_info_storage_2 (Utilities|Casting|CastToGI_InfoStorage (Game|GetGameInstance))
      (:then
        (Variables|/Game/Blueprints/GI_InfoStorage.GI_InfoStorage_C|SetGameWinner _asgi_info_storage_2 _winner1)
        (Variables|/Game/Blueprints/GI_InfoStorage.GI_InfoStorage_C|SetGamewinnerID _asgi_info_storage_2 (PlayerState|GetUniqueID _winner1)))
      (:CastFailed
        _))
    (bind _output_get (Variables|Default|SetGameWon? true))
    (bind _outactors (Actor|GetAllActorsOfClass "/Game/Variant_Combat/Blueprints/BP_CombatPlayerController.BP_CombatPlayerController_C"))
    (for _array_element _outactors
      (Default|FinalScoreboard _array_element _winner1))
    (return _output_get)
    (else
      (return false))))

(fn WhoWontheGame?
  (bind _asbp_game_state (Utilities|Casting|CastToBP_GameState (Game|GetGameState)))
  (for _array_element (Variables|/Script/Engine.GameStateBase|GetPlayerArray _asbp_game_state)
    (bind _asbp_player_state (Utilities|Casting|CastToBP_PlayerState _array_element))
    (if (> (Variables|/Game/Blueprints/GameInfo/BP_PlayerState.BP_PlayerState_C|GetWins _asbp_player_state) (LocalVariables|GetBestScore))
      (LocalVariables|SetBestScore (Variables|/Game/Blueprints/GameInfo/BP_PlayerState.BP_PlayerState_C|GetWins _asbp_player_state))
      (Utilities|Array|Clear (LocalVariables|GetTopPlayers))
      (LocalVariables|SetWinner _asbp_player_state)
      (Utilities|Array|Add (LocalVariables|GetTopPlayers) _asbp_player_state)
      (elif (== (Variables|/Game/Blueprints/GameInfo/BP_PlayerState.BP_PlayerState_C|GetWins _asbp_player_state) (LocalVariables|GetBestScore))
        (Utilities|Array|Add (LocalVariables|GetTopPlayers) _asbp_player_state))))
  (if (== (Utilities|Array|Length (LocalVariables|GetTopPlayers)) 1)
    (return (LocalVariables|GetWinner))
    (elif (> (Utilities|Array|Length (LocalVariables|GetTopPlayers)) 1)
      (for _array_element_2 (LocalVariables|GetTopPlayers)
        (bind _asbp_player_state_2 (Utilities|Casting|CastToBP_PlayerState _array_element_2))
        (if (> (Variables|/Game/Blueprints/GameInfo/BP_PlayerState.BP_PlayerState_C|GetOverallKills _asbp_player_state_2) (LocalVariables|GetBestKills))
          (LocalVariables|SetBestKills (Variables|/Game/Blueprints/GameInfo/BP_PlayerState.BP_PlayerState_C|GetOverallKills _asbp_player_state_2))
          (LocalVariables|SetWinner _asbp_player_state_2)))
      (return (LocalVariables|GetWinner))
      (else
        (return 0)))))

(fn OnRepRoundsNeededtoEndGame
  (bind _asbp_game_state (Utilities|Casting|CastToBP_GameState (Game|GetGameState)))
  (Variables|/Game/Blueprints/GameInfo/BP_GameState.BP_GameState_C|SetRoundsNeededToEndGame _asbp_game_state (Variables|Default|GetRoundsNeededToEndGame)))

(fn Start
  (Variables|Default|SetRoundStarted? true)
  (bind _returnvalue (Game|GetCurrentLevelName true))
  (if (Utilities|String|Contains _returnvalue "colosseum")
    (bind _outactors (Actor|GetAllActorsOfClass "/Game/Blueprints/BP_Cage.BP_Cage_C"))
    (for _array_element _outactors
      (Utilities|IsValid _array_element
        (:Is%20Valid
          (Class|BPIRoundStart|Start(Message) _array_element))))
    (bind _outactors_2 (Actor|GetAllActorsOfClass "/Game/Variant_Combat/Blueprints/BP_CombatPlayerController.BP_CombatPlayerController_C"))
    (for _array_element_2 _outactors_2
      (Default|EnableInputs _array_element_2))
    (return)
    (else
      (bind _outactors_3 (Actor|GetAllActorsOfClass "/Game/Variant_Combat/Blueprints/BP_CombatPlayerController.BP_CombatPlayerController_C"))
      (for _array_element_3 _outactors_3
        (Default|EnableInputs _array_element_3))
      (return))))