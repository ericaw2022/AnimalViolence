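; House actor with replicated base and roof materials and a door that can swing open at random.
; On BeginPlay the authority sets both color indices, whose RepNotifies apply the color materials to the house mesh slots.
; DoorOpen rolls a random number against HouseNumber, then a timeline rotates the door, with a delayed play or reverse driven by a toggled flag.
; Nothing connected in this graph calls DoorOpen.
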(event Custom|ChangeHouseColors
  (Variables|Default|SetBaseColorIndex 0)
  (Variables|Default|SetRoofColorIndex 0))

(event Custom|DoorOpen
  ;[0.15 0.15 0.15 0.5] Door Open Event
  (Variables|Default|SetRandomDoorNum (Math|Random|RandomIntegerinRange 1 5))
  (if (== (Variables|Default|GetHouseNumber) (Variables|Default|GetRandomDoorNum))
    (bind _doorrotate (Timeline|Timeline Play)
      (:Update
        (Transformation|SetRelativeRotation (Variables|Default|GetHouse_Door1) (Math|Rotator|MakeRotator 0.0 0.0 _doorrotate) false false)
        (if (Variables|Default|GetDoorOpen?)
          (Variables|Default|SetDoorOpen? false)
          (else
            (Variables|Default|SetDoorOpen? true)))
        (Utilities|FlowControl|Delay 1e+01)
        (if (Variables|Default|GetDoorOpen?)
          (Timeline|Timeline Reverse)
          (else
            (Timeline|Timeline Play))))
      (:Finished
        (if (Variables|Default|GetDoorOpen?)
          _)))))

(event EventBeginPlay
  (Networking|SwitchHasAuthority
    (:Authority
      (CallFunction|ChangeHouseColors))))

(event Collision|EventActorBeginOverlap
  (params (OtherActor :type Actor%20Object%20Reference)))

(event EventTick
  (params (DeltaSeconds :type Float%20%28single-precision%29)))

(fn ConstructionScript)

(fn OnRepHouseBaseColor)

(fn OnRepHouseRoofColor)

(fn OnRepRoofColorIndex
  ;[0.15 0.15 0.15 0.5] House Roof Color
  (Rendering|Material|SetMaterial (Variables|Default|GetHouse_Reg2) 0 (Variables|Default|GetHouseRoofColor)))

(fn OnRepBaseColorIndex
  ;[0.15 0.15 0.15 0.5] House Base Color
  (Rendering|Material|SetMaterial (Variables|Default|GetHouse_Reg2) 5 (Variables|Default|GetHouseBaseColor)))