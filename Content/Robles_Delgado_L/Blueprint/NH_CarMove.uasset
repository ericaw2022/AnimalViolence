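; NH_CarMove is a moving car hazard that repeatedly drives to a destination and damages combat characters it hits.
; On the server, BeginPlay starts an endless loop that moves the root to CarDestination over a random duration, waits a random delay, then teleports by the TPLocation offset.
; A Box overlap deals very high damage to any BP_CombatCharacter, without an authority check.
; A similar branch for BP_CombatEnemy is disconnected.
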(event OnComponentBeginOverlap(Box)
  (params (OverlappedComponent :type Primitive%20Component%20Object%20Reference) (OtherActor :type Actor%20Object%20Reference) (OtherComp :type Primitive%20Component%20Object%20Reference) (OtherBodyIndex :type Integer) (bFromSweep :type Boolean) (SweepResult :type Hit%20Result%20Structure%20%28by%20ref%29))
  (bind _asbp_combat_character (Utilities|Casting|CastToBP_CombatCharacter OtherActor))
  (Game|Damage|ApplyDamage _asbp_combat_character 999.0 0 0))

(event Custom|CarMovement
  (Components|MoveComponentTo (Variables|Transformation|GetRootComponent) (Variables|Default|GetCarDestination) (Transformation|GetActorRotation) false false (Math|Random|RandomFloatinRange (Variables|Default|GetCarSpeedMin) (Variables|Default|GetCarSpeedMax)) false :!label _label)
  (Utilities|FlowControl|Delay (Math|Random|RandomFloatinRange (Variables|Default|GetDelayMin) (Variables|Default|GetDelayMax)))
  (Transformation|Teleport (+ (Transformation|GetActorLocation) (Variables|Default|GetTPLocation)) (Transformation|GetActorRotation))
  (goto _label))

(event EventBeginPlay
  (Networking|SwitchHasAuthority
    (:Authority
      (CallFunction|CarMovement))))

(event EventTick
  (params (DeltaSeconds :type Float%20%28single-precision%29)))

(fn ConstructionScript)